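; Black hole magic projectile that flies straight without gravity while pulling in its surroundings through a negative-strength radial force, ignoring its instigator.
; BeginPlay configures both the movement and radial force components.
; Sphere overlaps with actors other than the instigator add BP_SActionEffectBlack through SActionComponent unless the Debuff.Black tag is active.
; The projectile destroys itself when the overlapped component simulates physics.
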(event OnComponentBeginOverlap(m_SphereCom)
  (params (OverlappedComponent :type Primitive%20Component%20Object%20Reference) (OtherActor :type Actor%20Object%20Reference) (OtherComp :type Primitive%20Component%20Object%20Reference) (OtherBodyIndex :type Integer) (bFromSweep :type Boolean) (SweepResult :type Hit%20Result%20Structure%20%28by%20ref%29))
  (bind _returnvalue (Game|GetInstigator))
  (bind _returnvalue_2 (Actor|GetComponentbyClass OtherActor "/Script/UnrealARPG.SActionComponent"))
  (if (!= OtherActor _returnvalue)
    (Utilities|FlowControl|Sequence
      (:then_0
        (Utilities|IsValid _returnvalue_2
          (:Is%20Valid
            (bind _returnvalue_3 (Class|SActionComponent|IsAciveTag _returnvalue_2 "(TagName=\"Debuff.Black\")"))
            (if (not _returnvalue_3)
              (Class|SActionComponent|AddAction _returnvalue_2 _returnvalue "/Game/BluePrints/Actions/BP_SActionEffectBlack.BP_SActionEffectBlack_C")))))
      (:then_1
        (if (Physics|IsSimulatingPhysics OtherComp "None")
          (Actor|DestroyActor))))))

(event EventBeginPlay
  (bind _m_pjmovecom (Variables|Default|Getm_PjMoveCom))
  (bind _sradialforce (Variables|Default|GetSRadialForce))
  (Variables|/Script/UnrealARPG.SRadialForceComponent|SetInstigator (Variables|Default|GetSRadialForce) (Game|GetInstigator))
  (Variables|/Script/Engine.ProjectileMovementComponent|SetProjectileGravityScale _m_pjmovecom 0.0)
  (Variables|/Script/Engine.ProjectileMovementComponent|SetbInitialVelocityInLocalSpace _m_pjmovecom true)
  (Variables|/Script/Engine.ProjectileMovementComponent|SetbRotationFollowsVelocity _m_pjmovecom true)
  (Variables|/Script/Engine.ProjectileMovementComponent|SetInitialSpeed (Variables|Default|Getm_PjMoveCom) 1e+03)
  (Variables|/Script/UnrealARPG.SRadialForceComponent|SetbIgnoreInstigator _sradialforce true)
  (Variables|/Script/Engine.RadialForceComponent|SetRadius _sradialforce 8e+02)
  (Variables|/Script/Engine.RadialForceComponent|SetForceStrength _sradialforce -2e+06))

(fn ConstructionScript)