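; BP_SActionEffectBlack is an action effect that shows a black screen overlay to the affected player while it is active.
; On start it casts the owning component's owner to BPSCharacter and, only if locally controlled, creates the BlackEffect widget for that player's controller and adds it to the viewport.
; On stop it removes the stored widget if it is still valid.
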(event EventStartAction
  (params (Instigator :type Actor%20Object%20Reference))
  (|CallParentFunction Instigator)
  (bind _asbpscharacter (Utilities|Casting|CastToBPSCharacter (Components|GetOwner (Class|SAction|GetOwningComponent))))
  (if (Pawn|IsLocallyControlled _asbpscharacter)
    (bind _as玩家控制器 (Utilities|Casting|CastToPlayerController (Pawn|GetController _asbpscharacter)))
    (bind _returnvalue (UserInterface|CreateWidget "/Game/UI/BlackEffect.BlackEffect_C" _as玩家控制器))
    (bind _output_get (Variables|Default|SetBlackUI _returnvalue))
    (UserInterface|Viewport|AddtoViewport _output_get 0)))

(event EventStopAction
  (params (Instigator :type Actor%20Object%20Reference))
  (bind _blackui (Variables|Default|GetBlackUI))
  (|CallParentFunction Instigator)
  (Utilities|IsValid _blackui
    (:Is%20Valid
      (Widget|RemovefromParent _blackui))))