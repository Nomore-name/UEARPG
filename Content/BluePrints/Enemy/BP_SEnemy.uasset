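; Enemy character Blueprint that stores its target and a can-add-health flag in the AI Blackboard.
; Pawn sensing sets the target and shows a notice widget for new sightings; health changes from non-enemy pawns also retarget it.
; Health changes spawn colored floating numbers, and non-lethal damage creates a single attached health bar.
; On death it ragdolls the mesh, disables capsule collision, stops AI logic and expires after a delay.
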(event OnHealthChanged(SAttribute)
  (params (InstigatorActor :type Actor%20Object%20Reference) (OwingComp :type S%20Attribute%20Component%20Object%20Reference) (NewHealth :type Float%20%28single-precision%29) (ChangeValue :type Float%20%28single-precision%29))
  (bind _mesh (Variables|Character|GetMesh))
  (Utilities|FlowControl|Sequence
    (:then_0
      ;[1 1 1] UI显示
      (bind _returnvalue (UserInterface|CreateWidget "/Game/UI/ActorHealthNum.ActorHealthNum_C" 0 (Utilities|Text|ToText(Float) ChangeValue "HalfToEven") self (select (> ChangeValue 0.0) (Variables|Default|GetText%20Color%20Green) (Variables|Default|GetText%20Color%20Red))))
      (UserInterface|Viewport|AddtoViewport _returnvalue 0))
    (:then_1
      ;[1 1 1] 设置目标
      (if (!= InstigatorActor self)
        (bind _aspawn (Utilities|Casting|CastToPawn InstigatorActor))
        (if (not (Actor|ActorHasTag _aspawn "Enemy"))
          (CallFunction|SetTarget _aspawn))))
    (:then_2
      ;[1 1 1] 死亡
      (if (and (< ChangeValue 0.0) (<= NewHealth 0.0))
        (Collision|SetCollisionEnabled _mesh "QueryAndPhysics")
        (Class|SkeletalMeshComponent|SetAllBodiesSimulatePhysics _mesh true)
        (Collision|SetCollisionEnabled (Variables|Collision|GetCapsuleComponent) "NoCollision")
        (bind _asai控制器 (Utilities|Casting|CastToAIController (Pawn|GetController)))
        (AI|Logic|StopLogic (Variables|/Script/AIModule.AIController|GetBrainComponent _asai控制器) "Death")
        (Actor|SetLifeSpan 1e+01)))
    (:then_3
      ;[1 1 1] 添加血条
      (if (and (< ChangeValue 0.0) (> NewHealth 0.0))
        (Utilities|IsValid (Variables|Default|GetActiveHealthBar)
          (:Is%20Not%20Valid
            (bind _returnvalue_2 (UserInterface|CreateWidget "/Game/UI/EnemyHealthBar.EnemyHealthBar_C"))
            (bind _output_get (Variables|Default|SetActiveHealthBar _returnvalue_2))
            (Variables|/Script/UnrealARPG.SUserWidgetEnemyHealthBar|Setm_AttachedActor _output_get self)
            (UserInterface|Viewport|AddtoViewport _output_get 0)))))))

(event OnSeePawn(PawnSensing)
  (params (Pawn :type Pawn%20Object%20Reference))
  (bind _targetpawn (CallFunction|GetTarget))
  (if (!= _targetpawn Pawn)
    (CallFunction|SetTarget Pawn)
    (bind _returnvalue (UserInterface|CreateWidget "/Game/UI/SUserWidgetNotice.SUserWidgetNotice_C" 0 self))
    (UserInterface|Viewport|AddtoViewport _returnvalue 0)))

(event Custom|SetTarget
  (params (Pawn :type Pawn%20Object%20Reference))
  (AI|Components|Blackboard|SetValueasObject (Variables|/Script/AIModule.AIController|GetBlackboard (AI|GetAIController (Components|GetOwner))) (Variables|Default|GetFNameTargetActor) Pawn))

(event Custom|SetCanAddHealth
  (params (CanAddHealth :type Boolean))
  (AI|Components|Blackboard|SetValueasBool (Variables|/Script/AIModule.AIController|GetBlackboard (AI|GetAIController (Components|GetOwner))) (Variables|Default|GetFNameHealth) CanAddHealth))

(event EventBeginPlay
  (Collision|SetCollisionResponsetoChannel (Variables|Collision|GetCapsuleComponent) "ECC_WorldDynamic" "ECR_Ignore")
  (Variables|/Script/Engine.PrimitiveComponent|SetbGenerateOverlapEvents (Variables|Character|GetMesh) true))

(fn ConstructionScript)

(fn GetTarget
  (bind _aspawn (Utilities|Casting|CastToPawn (AI|Components|Blackboard|GetValueasObject (Variables|/Script/AIModule.AIController|GetBlackboard (AI|GetAIController (Components|GetOwner))) (Variables|Default|GetFNameTargetActor)))
    (:then
      _)
    (:CastFailed
      _))
  (return _aspawn))