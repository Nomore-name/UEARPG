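; BP_Fort is a turret-like fort that shoots magic projectiles at the player while it has health left.
; Tick runs through a one-second Delay, throttling fire to about once per second, aimed from its Sphere at the player pawn.
; It fires only when the world-space look-at yaw lies within a fixed forward arc.
; Health changes from its SAttribute component spawn an attached health-number widget while health stays above zero.
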(event OnHealthChanged(SAttribute)
  (params (InstigatorActor :type Actor%20Object%20Reference) (OwingComp :type S%20Attribute%20Component%20Object%20Reference) (NewHealth :type Float%20%28single-precision%29) (ChangeValue :type Float%20%28single-precision%29))
  (bind _sattribute (Variables|Default|GetSAttribute))
  (bind _m_health (Variables|/Script/UnrealARPG.SAttributeComponent|Getm_Health _sattribute))
  (if (> _m_health 0.0)
    (bind _returnvalue (UserInterface|CreateWidget "/Game/UI/ActorHealthNum.ActorHealthNum_C" 0 (Utilities|Text|ToText(Float) _m_health "HalfToEven") self))
    (UserInterface|Viewport|AddtoViewport _returnvalue 0)))

(event EventTick
  (params (DeltaSeconds :type Float%20%28single-precision%29))
  (bind _returnvalue (Game|Player|GetPlayerPawn 0))
  (bind _sphere (Variables|Default|GetSphere))
  (bind _returnvalue_2 (Transformation|GetActorLocation _returnvalue))
  (bind _returnvalue_3 (Transformation|GetWorldLocation _sphere))
  (bind _returnvalue_4 (Math|Rotator|FindLookatRotation _returnvalue_3 _returnvalue_2))
  (bind _yaw (Math|Rotator|BreakRotator _returnvalue_4))
  (Utilities|FlowControl|Delay 1.0)
  (if (Math|Boolean|ANDBoolean (< _yaw 8e+01) (> _yaw -8e+01) (> (Variables|/Script/UnrealARPG.SAttributeComponent|Getm_Health (Variables|Default|GetSAttribute)) 0.0))
    (Game|SpawnActorfromClass "/Game/BluePrints/Projectile/BP_SProjectileMagic.BP_SProjectileMagic_C" (Math|Transform|MakeTransform _returnvalue_3 _returnvalue_4) "Undefined" "MultiplyWithRoot" 0 0)))

(fn ConstructionScript)